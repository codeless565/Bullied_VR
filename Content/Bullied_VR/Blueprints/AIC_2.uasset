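; AI controller that runs behavior tree BT_2 for a TestAI_2 pawn in the Bullied_VR project.
; On BeginPlay it seeds the blackboard's StartPosition and EndPosition.
; With IsRandomGoal set, these are the pawn's location and a random reachable point nearby; otherwise they come from the pawn's StartPos and EndPos.
; Both paths also cache the player's BP_MotionControllerPawnFPS in PlayerMCRef.
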(event `self.ReceiveBeginPlay`
  (bind _returnvalue (`self.K2_GetPawn`))
  (bind _returnvalue_2 (`AIBlueprintHelperLibrary.GetBlackboard` null))
  (bind _returnvalue_3 (`AIBlueprintHelperLibrary.GetBlackboard` null))
  (bind _returnvalue_4 (`self.K2_GetActorLocation` _returnvalue))
  (`self.RunBehaviorTree` "/Game/Bullied_VR/Blueprints/BT_2.BT_2")
  (bind _astest_ai_2 (cast `/Game/Bullied_VR/Blueprints/TestAI_2` _returnvalue))
  (if (`/Game/Bullied_VR/Blueprints/TestAI_2.IsRandomGoal` _astest_ai_2)
    (`BlackboardComponent.SetValueAsVector` _returnvalue_3 "StartPosition" _returnvalue_4)
    (`BlackboardComponent.SetValueAsVector` _returnvalue_3 "EndPosition" (`NavigationSystem.K2_GetRandomReachablePointInRadius` _returnvalue_4 500.0))
    (bind _asbp_motion_controller_pawn_fps (cast `/Game/Bullied_VR/Blueprints/BP_MotionControllerPawnFPS` (`self.K2_GetPawn` (`GameplayStatics.GetPlayerController` 0))))
    (set `self.PlayerMCRef` _asbp_motion_controller_pawn_fps)
    (else
      (`BlackboardComponent.SetValueAsVector` _returnvalue_2 "StartPosition" (`/Game/Bullied_VR/Blueprints/TestAI_2.StartPos` _astest_ai_2))
      (`BlackboardComponent.SetValueAsVector` _returnvalue_2 "EndPosition" (`/Game/Bullied_VR/Blueprints/TestAI_2.EndPos` _astest_ai_2))
      (bind _asbp_motion_controller_pawn_fps_2 (cast `/Game/Bullied_VR/Blueprints/BP_MotionControllerPawnFPS` (`self.K2_GetPawn` (`GameplayStatics.GetPlayerController` 0))))
      (set `self.PlayerMCRef` _asbp_motion_controller_pawn_fps_2))))

(fn `UserConstructionScript`)