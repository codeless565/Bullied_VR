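; Choice trigger actor that presents a one-time list of selectable choices to the VR player through the motion controller pawn's choice widget.
; ActivateChoice registers itself on the pawn, disables motion and fills the ChoiceList from the passed array.
; ChangeChoiceUp and ChangeChoiceDown move the highlight within list bounds, and SelectChoice submits the index and restores motion.
; Once triggered, Tick watches for the choice ending, then hides and finishes the widget after a short delay.
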(event `self.ReceiveTick`
  (params (DeltaSeconds :type "Float (single-precision)"))
  (bind _pchoicewidget (`self.PChoiceWIdget`))
  ;[1 1 1] Check if player Trigger Choice Selection
  (if (`self.Triggered`)
    (if (not (`/Game/Bullied_VR/Blueprints/MotionControllerPawnFPS.InChoice` (`self.PlayerMCRef`)))
      (`KismetSystemLibrary.Delay` 1.0)
      (`Widget.SetVisibility` _pchoicewidget "Hidden")
      (bind _aschoice_list (cast `/Game/Bullied_VR/Blueprints/ChoiceList` _pchoicewidget))
      (`/Game/Bullied_VR/Blueprints/ChoiceList.OnFinish` _aschoice_list))))

(fn `ActivateChoice`
  (params (ChoiceArray :type "Array of /Game/Bullied_VR/Blueprints/ChoiceInfo Structure"))
  (bind _playermcref (`self.PlayerMCRef`))
  (bind _playermcref_2 (`self.PlayerMCRef`))
  (bind _returnvalue (`Controller.K2_GetPawn` (`GameplayStatics.GetPlayerController` 0)))
  (bind _choicewidget (`/Game/Bullied_VR/Blueprints/MotionControllerPawnFPS.ChoiceWidget` _playermcref))
  ;[1 1 1] Render Choice selection on screen
  (if (`self.Triggered`)
    _
    (elif (`KismetMathLibrary.ClassIsChildOf` (`GameplayStatics.GetObjectClass` _returnvalue) "/Game/Bullied_VR/Blueprints/MotionControllerPawnFPS.MotionControllerPawnFPS_C")
      (bind _asmotion_controller_pawn_fps (cast `/Game/Bullied_VR/Blueprints/MotionControllerPawnFPS` _returnvalue))
      (set `self.PlayerMCRef` _asmotion_controller_pawn_fps)
      (set `self.PChoiceWIdget` _choicewidget)
      (set `/Game/Bullied_VR/Blueprints/MotionControllerPawnFPS.ChoiceTriggerBox` self _playermcref)
      (`Widget.SetVisibility` _choicewidget "Visible")
      (set `/Game/Bullied_VR/Blueprints/MotionControllerPawnFPS.InChoice` true _playermcref_2)
      (set `/Game/Bullied_VR/Blueprints/MotionControllerPawnFPS.DisableMotion` true _playermcref_2)
      (bind _aschoice_list (cast `/Game/Bullied_VR/Blueprints/ChoiceList` _choicewidget))
      (set `/Game/Bullied_VR/Blueprints/ChoiceList.ChoiceInfoArray` ChoiceArray _aschoice_list)
      (`/Game/Bullied_VR/Blueprints/ChoiceList.OnCreate` _aschoice_list)
      (bind _vbox (`/Game/Bullied_VR/Blueprints/ChoiceList.VBox` _aschoice_list))
      (set `self.PChoiceWidgetVBox` _vbox)
      (bind _aschoice_selection (cast `/Game/Bullied_VR/Blueprints/ChoiceSelection` (`PanelWidget.GetChildAt` _vbox 0)))
      (set `/Game/Bullied_VR/Blueprints/ChoiceSelection.Selected` true _aschoice_selection)
      (set `self.Triggered` true)
      (`/Game/Bullied_VR/Blueprints/ChoiceList.ChangeChoice` _aschoice_list 0))))

(fn `ChangeChoiceDown`
  (bind _choiceindex (`self.ChoiceIndex`))
  (bind _pchoicewidgetvbox (`self.PChoiceWidgetVBox`))
  (bind _choiceindex_2 (`self.ChoiceIndex`))
  (bind _aschoice_list (cast `/Game/Bullied_VR/Blueprints/ChoiceList` (`self.PChoiceWIdget`)))
  (`/Engine/EditorBlueprintResources/StandardMacros.CompareInt` _choiceindex (- (`PanelWidget.GetChildrenCount` _pchoicewidgetvbox) 1)
    (:`<`
      (bind _aschoice_selection (cast `/Game/Bullied_VR/Blueprints/ChoiceSelection` (`PanelWidget.GetChildAt` _pchoicewidgetvbox _choiceindex)))
      (set `/Game/Bullied_VR/Blueprints/ChoiceSelection.Selected` false _aschoice_selection)
      (`/Game/Bullied_VR/Blueprints/ChoiceList.ChangeChoice` _aschoice_list _choiceindex_2)
      (bind _result (`/Engine/EditorBlueprintResources/StandardMacros.IncrementInt` _choiceindex_2)
        (:`  `
          (bind _aschoice_selection_2 (cast `/Game/Bullied_VR/Blueprints/ChoiceSelection` (`PanelWidget.GetChildAt` (`self.PChoiceWidgetVBox`) _result)))
          (set `/Game/Bullied_VR/Blueprints/ChoiceSelection.Selected` true _aschoice_selection_2)
          (`/Game/Bullied_VR/Blueprints/ChoiceList.ChangeChoice` _aschoice_list _result))))))

(fn `ChangeChoiceUp`
  (bind _choiceindex (`self.ChoiceIndex`))
  (bind _choiceindex_2 (`self.ChoiceIndex`))
  (bind _aschoice_list (cast `/Game/Bullied_VR/Blueprints/ChoiceList` (`self.PChoiceWIdget`)))
  (`/Engine/EditorBlueprintResources/StandardMacros.CompareInt` _choiceindex
    (:`>`
      (bind _aschoice_selection (cast `/Game/Bullied_VR/Blueprints/ChoiceSelection` (`PanelWidget.GetChildAt` (`self.PChoiceWidgetVBox`) _choiceindex)))
      (set `/Game/Bullied_VR/Blueprints/ChoiceSelection.Selected` false _aschoice_selection)
      (`/Game/Bullied_VR/Blueprints/ChoiceList.ChangeChoice` _aschoice_list _choiceindex_2)
      (bind _result (`/Engine/EditorBlueprintResources/StandardMacros.DecrementInt` _choiceindex_2)
        (:`  `
          (bind _aschoice_selection_2 (cast `/Game/Bullied_VR/Blueprints/ChoiceSelection` (`PanelWidget.GetChildAt` (`self.PChoiceWidgetVBox`) _result)))
          (set `/Game/Bullied_VR/Blueprints/ChoiceSelection.Selected` true _aschoice_selection_2)
          (`/Game/Bullied_VR/Blueprints/ChoiceList.ChangeChoice` _aschoice_list _result))))))

(fn `SelectChoice`
  (bind _playermcref (`self.PlayerMCRef`))
  (bind _aschoice_list (cast `/Game/Bullied_VR/Blueprints/ChoiceList` (`self.PChoiceWIdget`)))
  (`/Game/Bullied_VR/Blueprints/ChoiceList.SelectChoice` _aschoice_list (`self.ChoiceIndex`))
  (set `/Game/Bullied_VR/Blueprints/MotionControllerPawnFPS.InChoice` false _playermcref)
  (set `/Game/Bullied_VR/Blueprints/MotionControllerPawnFPS.DisableMotion` false _playermcref))

(fn `UserConstructionScript`)