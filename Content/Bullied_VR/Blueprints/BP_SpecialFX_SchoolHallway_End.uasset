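; BP_SpecialFX_SchoolHallway_End is a trigger box that ends the school hallway special effects by calling ResetSkyLight on its linked SPFX_Start actor.
; It destroys itself on BeginPlay without that reference; otherwise it starts with collision and tick off, exposing SetEnable to arm it.
; While enabled, Tick polls the box for overlap with the player, then triggers the reset and destroys the actor.
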(event `self.ReceiveBeginPlay`
  (`/Engine/EditorBlueprintResources/StandardMacros.IsValid` (`self.SPFXStartRef`)
    (:`Is Valid`
      (`self.SetDisable`))
    (:`Is Not Valid`
      (`self.K2_DestroyActor`))))

(event `self.ReceiveTick`
  (params (DeltaSeconds :type "Float (single-precision)"))
  ;[1 1 1] When Player Touch this trigger box, Call function in SPFX_Start to reset all effects
  (if (`PrimitiveComponent.IsOverlappingActor` (`self.BoxCollision`) (`self.PlayerMC_Ref`))
    (`/Game/Bullied_VR/Blueprints/BP_SpecialFX_SchoolHallway_Start.ResetSkyLight` (`self.SPFXStartRef`))
    (`self.K2_DestroyActor`)))

(fn `SetDisable`
  (`self.SetActorEnableCollision` false)
  (`self.SetActorTickEnabled` false))

(fn `SetEnable`
  (`self.SetActorEnableCollision` true)
  (`self.SetActorTickEnabled` true))

(fn `UserConstructionScript`)