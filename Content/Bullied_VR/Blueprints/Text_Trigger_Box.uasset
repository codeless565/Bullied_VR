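; Text trigger box for a VR game that shows subtitles on the player pawn's widget for voiced cutscenes and interaction text.
; StartSubtitleSequence loads lines from a string table, locks pawn motion, then Tick shows the next line and plays the next clip whenever audio stops.
; StartInteractionText registers the box with the pawn, and IterateText advances a preset text array one line per call.
; Both modes restore motion and unregister after the last line.
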(event `self.ReceiveBeginPlay`)

(event `self.ReceiveTick`
  (params (DeltaSeconds :type "Float (single-precision)"))
  (bind _audioplayer (`self.AudioPlayer`))
  (bind _audioindex (`self.AudioIndex`))
  (if (`self.IsPlayingCutscene`)
    (if (not (`AudioComponent.IsPlaying` _audioplayer))
      (`self.PlayCutsceneSubtitle`)
      (`AudioComponent.SetSound` _audioplayer (`|GetArrayItem` (`self.Audio`) _audioindex))
      (`AudioComponent.Play` _audioplayer 0.0)
      (`/Engine/EditorBlueprintResources/StandardMacros.CompareInt` _audioindex (- (`KismetArrayLibrary.Array_Length` (`self.Audio`)) 1)
        (:`<`
          (`/Engine/EditorBlueprintResources/StandardMacros.IncrementInt` (`self.AudioIndex`)))))))

(fn `IterateText`
  (bind _interacttextarray (`self.InteractTextArray`))
  (bind _subtitleindex (`self.SubtitleIndex`))
  (bind _mpawnref (`self.MPawnRef`))
  (bind _assubtitle (cast `/Game/Bullied_VR/Blueprints/Subtitle` (`self.PSubtitleRef`)))
  (`/Engine/EditorBlueprintResources/StandardMacros.CompareInt` _subtitleindex (- (`KismetArrayLibrary.Array_Length` _interacttextarray) 1)
    (:`>`
      (set `/Game/Bullied_VR/Blueprints/MotionControllerPawnFPS.DisableMotion` false _mpawnref)
      (`/Game/Bullied_VR/Blueprints/Subtitle.DisplaySubtitleText` _assubtitle false)
      (set `self.SubtitleIndex` 0)
      (set `/Game/Bullied_VR/Blueprints/MotionControllerPawnFPS.TextTriggerBox` null (`self.MPawnRef`)))
    (:`==`
      (`/Game/Bullied_VR/Blueprints/Subtitle.SetSubtitleText` _assubtitle (`|GetArrayItem` _interacttextarray _subtitleindex) :!label _label)
      (`/Game/Bullied_VR/Blueprints/Subtitle.DisplaySubtitleText` _assubtitle true)
      (`/Engine/EditorBlueprintResources/StandardMacros.IncrementInt` _subtitleindex
        (:`  `
          (set `/Game/Bullied_VR/Blueprints/MotionControllerPawnFPS.DisableMotion` true _mpawnref))))
    (:`<`
      (goto _label))))

(fn `PlayCutsceneSubtitle`
  (bind _subtitletextarray (`self.SubtitleTextArray`))
  (bind _subtitleindex (`self.SubtitleIndex`))
  (bind _assubtitle (cast `/Game/Bullied_VR/Blueprints/Subtitle` (`self.PSubtitleRef`)))
  (`/Engine/EditorBlueprintResources/StandardMacros.CompareInt` _subtitleindex (- (`KismetArrayLibrary.Array_Length` _subtitletextarray) 1)
    (:`>`
      (set `/Game/Bullied_VR/Blueprints/MotionControllerPawnFPS.DisableMotion` false (`self.MPawnRef`))
      (`/Game/Bullied_VR/Blueprints/Subtitle.DisplaySubtitleText` _assubtitle false)
      (set `self.SubtitleIndex` 0)
      (set `/Game/Bullied_VR/Blueprints/MotionControllerPawnFPS.TextTriggerBox` null (`self.MPawnRef`))
      (set `self.IsPlayingCutscene` false))
    (:`==`
      (`/Game/Bullied_VR/Blueprints/Subtitle.SetSubtitleText` _assubtitle (`|GetArrayItem` _subtitletextarray _subtitleindex) :!label _label)
      (`/Game/Bullied_VR/Blueprints/Subtitle.DisplaySubtitleText` _assubtitle true)
      (`/Engine/EditorBlueprintResources/StandardMacros.IncrementInt` _subtitleindex))
    (:`<`
      (goto _label))))

(fn `SetStringTable`
  (params (`String Table Name` :type Name))
  (bind _subtitletextarray (`self.SubtitleTextArray`))
  (`KismetArrayLibrary.Array_Clear` _subtitletextarray)
  (for _array_element (`KismetStringTableLibrary.GetKeysFromStringTable` `String Table Name`)
    (`KismetArrayLibrary.Array_Add` _subtitletextarray (`KismetTextLibrary.Conv_TextToString` (`KismetTextLibrary.TextFromStringTable` `String Table Name` _array_element)))))

(fn `StartInteractionText`
  (bind _asmotion_controller_pawn_fps (cast `/Game/Bullied_VR/Blueprints/MotionControllerPawnFPS` (`Controller.K2_GetPawn` (`GameplayStatics.GetPlayerController` 0))))
  (set `/Game/Bullied_VR/Blueprints/MotionControllerPawnFPS.TextTriggerBox` self _asmotion_controller_pawn_fps)
  (set `self.PSubtitleRef` (`/Game/Bullied_VR/Blueprints/MotionControllerPawnFPS.SubtitleWidget` _asmotion_controller_pawn_fps))
  (set `self.MPawnRef` _asmotion_controller_pawn_fps))

(fn `StartSubtitleSequence`
  (params (`Audio Array` :type "Array of SoundWave Object Reference") (`String Table Name` :type Name))
  (`self.SetStringTable` `String Table Name`)
  (set `self.Audio` `Audio Array`)
  (set `self.IsPlayingCutscene` true)
  (bind _asmotion_controller_pawn_fps (cast `/Game/Bullied_VR/Blueprints/MotionControllerPawnFPS` (`Controller.K2_GetPawn` (`GameplayStatics.GetPlayerController` 0))))
  (set `/Game/Bullied_VR/Blueprints/MotionControllerPawnFPS.TextTriggerBox` self _asmotion_controller_pawn_fps)
  (set `self.PSubtitleRef` (`/Game/Bullied_VR/Blueprints/MotionControllerPawnFPS.SubtitleWidget` _asmotion_controller_pawn_fps))
  (set `self.MPawnRef` _asmotion_controller_pawn_fps)
  (set `/Game/Bullied_VR/Blueprints/MotionControllerPawnFPS.DisableMotion` true _asmotion_controller_pawn_fps))

(fn `UserConstructionScript`)