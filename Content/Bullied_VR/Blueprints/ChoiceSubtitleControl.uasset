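; ChoiceSubtitleControl is a Blueprint that triggers subtitle and choice sequences according to the player's checkpoint progress.
; ActivateSubtitle and ActivateChoice each read CheckpointIndex from Game_Instance and act only at one specific checkpoint.
; A match starts the first subtitle sequence through TTB or the first choice selection through CTB.
; The event graph is empty, so both functions depend on being called.
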(fn `ActivateChoice`
  (bind _asgame_instance (cast `/Game/Bullied_VR/Blueprints/Game_Instance` (`GameplayStatics.GetGameInstance`)))
  (`|ExecutionSequence`
    (:`then_0`
      (`/Engine/EditorBlueprintResources/StandardMacros.CompareInt` (`/Game/Bullied_VR/Blueprints/Game_Instance.Checkpoint_Index` _asgame_instance) 2
        (:`==`
          (`/Game/Bullied_VR/Blueprints/Choice_Trigger_Box.StartChoiceSelection` (`self.CTB`) (`self.Choice_1`)))))))

(fn `ActivateSubtitle`
  (bind _asgame_instance (cast `/Game/Bullied_VR/Blueprints/Game_Instance` (`GameplayStatics.GetGameInstance`)))
  (`|ExecutionSequence`
    (:`then_0`
      (`/Engine/EditorBlueprintResources/StandardMacros.CompareInt` (`/Game/Bullied_VR/Blueprints/Game_Instance.Checkpoint_Index` _asgame_instance) 1
        (:`==`
          (`/Game/Bullied_VR/Blueprints/Text_Trigger_Box.StartSubtitleSequence` (`self.TTB`) (`self.Subtitle_1`)))))))

(fn `UserConstructionScript`)