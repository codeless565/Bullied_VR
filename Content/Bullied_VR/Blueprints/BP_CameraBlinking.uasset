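; Blueprint that simulates the player blinking in a VR game by fading the player camera out and back in.
; CloseEye fades the camera to full and starts an elapsed timer, which Tick advances until it passes the blink time plus a short margin, then calls OpenEye to fade back.
; A negative elapsed time marks the timer as idle, and EndBlink sets it to stop a pending automatic reopen.
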(event `self.ReceiveBeginPlay`
  (set `self.f_ElapseTime` -1.0)
  (set `self.b_EyeClosed` false))

(event `self.ReceiveTick`
  (params (DeltaSeconds :type "Float (single-precision)"))
  (if (>= (`self.f_ElapseTime`) 0.0)
    (bind _output_get (set `self.f_ElapseTime` (+ (`self.f_ElapseTime`) (`GameplayStatics.GetWorldDeltaSeconds`))))
    (if (>= _output_get (+ (`self.f_BlinkTime`) 0.1))
      (if (`self.b_EyeClosed`)
        (`self.OpenEye`)))))

(fn `CloseEye`
  (`PlayerCameraManager.StartCameraFade` :`self` (`GameplayStatics.GetPlayerCameraManager` 0) :`FromAlpha` 0.0 :`ToAlpha` 1.0 :`Duration` (`self.f_BlinkTime`) :`bHoldWhenFinished` true)
  (set `self.f_ElapseTime` -0.0)
  (set `self.b_EyeClosed` true))

(fn `EndBlink`
  (set `self.f_ElapseTime` -1.0))

(fn `OpenEye`
  (`PlayerCameraManager.StartCameraFade` :`self` (`GameplayStatics.GetPlayerCameraManager` 0) :`FromAlpha` 1.0 :`ToAlpha` 0.0 :`Duration` (`self.f_BlinkTime`) :`bHoldWhenFinished` true)
  (set `self.f_ElapseTime` -1.0)
  (set `self.b_EyeClosed` false))

(fn `UserConstructionScript`)