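; Text box actor that runs subtitled cutscene dialogue and interaction text on the VR pawn's subtitle widget, optionally disabling player motion.
; Cutscene lines load from a string table, and Tick advances subtitle and audio together once no scene actor's audio is playing.
; When subtitles end, it either starts a choice selection or clears the cutscene manager's playing flag.
; Interaction text advances per IterateText call, pausing the AI's brain and turning it toward the player.
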(event `self.ReceiveBeginPlay`)

(event `self.ReceiveTick`
  (params (DeltaSeconds :type "Float (single-precision)"))
  (bind _audioindex (`self.AudioIndex`))
  (bind _audio (`self.Audio`))
  (bind _returnvalue (or (`self.IsInteractWithAudio`) (`self.IsPlayingCutscene`)))
  (bind (_audiofile _soundlocation) (break `/Game/Bullied_VR/Blueprints/SoundStruct` (`|GetArrayItem` _audio _audioindex)))
  (bind _audioplayer (`/Game/Bullied_VR/Blueprints/BP_EventTriggerBox.AudioPlayer` (`/Game/Bullied_VR/Blueprints/BP_ChoiceSubtitleManager.CurrEventTBox` (`self.CSManager`))))
  (bind _audioplayer_2 (`/Game/Bullied_VR/Blueprints/BP_SoundLocation.AudioPlayer` _soundlocation))
  (if _returnvalue
    (for _array_element (`self.ActorsInScene`)
      (bind _output_get (set `self.IsAudioPlaying` (`AudioComponent.IsPlaying` (`/Game/Bullied_VR/Blueprints/BP_SoundLocation.AudioPlayer` _array_element))))
      (if _output_get
        (break)))
    (if (not (`self.IsAudioPlaying`))
      (`self.PlayCutsceneSubtitle`)
      (if _returnvalue
        (`/Engine/EditorBlueprintResources/StandardMacros.IsValid` _audioplayer_2
          (:`Is Valid`
            (`AudioComponent.SetSound` _audioplayer _audiofile)
            (`AudioComponent.SetSound` _audioplayer_2 _audiofile)
            (`/Engine/EditorBlueprintResources/StandardMacros.IsValid` _audioplayer_2
              (:`Is Valid`
                (`AudioComponent.Play` _audioplayer_2 0.0))
              (:`Is Not Valid`
                (`AudioComponent.Play` _audioplayer 0.0)))
            (`/Engine/EditorBlueprintResources/StandardMacros.CompareInt` _audioindex (- (`KismetArrayLibrary.Array_Length` _audio) 1)
              (:`<`
                (`/Engine/EditorBlueprintResources/StandardMacros.IncrementInt` (`self.AudioIndex`)))))
          (:`Is Not Valid`
            (`AudioComponent.SetSound` _audioplayer _audiofile)))))))

(fn `IterateText`
  (bind _interactingai (`self.InteractingAI`))
  (bind _interacttextarray (`self.InteractTextArray`))
  (bind _subtitleindex (`self.SubtitleIndex`))
  (bind _mpawnref (`self.MPawnRef`))
  (bind _returnvalue (`AIBlueprintHelperLibrary.GetAIController` _interactingai))
  (bind _returnvalue_2 (`KismetSystemLibrary.IsValid` _interactingai))
  (if (`self.IsInteracting`)
    (`BrainComponent.StopLogic` (`AIController.BrainComponent` _returnvalue) "")
    (`self.K2_SetActorRotation` _interactingai (`KismetMathLibrary.FindLookAtRotation` (`self.K2_GetActorLocation` _interactingai) (`self.K2_GetActorLocation` (`Controller.K2_GetPawn` (`GameplayStatics.GetPlayerController` 0)))) false)
    (if _returnvalue_2
      _
      (else
        _))
    (bind _assubtitle (cast `/Game/Bullied_VR/Blueprints/Subtitle` (`self.PSubtitleRef`)))
    (`/Engine/EditorBlueprintResources/StandardMacros.CompareInt` _subtitleindex (- (`KismetArrayLibrary.Array_Length` _interacttextarray) 1)
      (:`>`
        (set `/Game/Bullied_VR/Blueprints/BP_MotionControllerPawnFPS.DisableMotion` false _mpawnref)
        (`/Game/Bullied_VR/Blueprints/Subtitle.DisplaySubtitleText` _assubtitle false)
        (set `self.SubtitleIndex` 0)
        (if _returnvalue_2
          (`BrainComponent.RestartLogic` (`AIController.BrainComponent` _returnvalue))
          (set `self.InteractingAI` null))
        (set `self.IsInteracting` false))
      (:`==`
        (`/Game/Bullied_VR/Blueprints/Subtitle.SetSubtitleText` _assubtitle (`|GetArrayItem` _interacttextarray _subtitleindex) :!label _label)
        (`/Game/Bullied_VR/Blueprints/Subtitle.DisplaySubtitleText` _assubtitle true)
        (`/Engine/EditorBlueprintResources/StandardMacros.IncrementInt` _subtitleindex
          (:`  `
            (set `/Game/Bullied_VR/Blueprints/BP_MotionControllerPawnFPS.DisableMotion` true _mpawnref))))
      (:`<`
        (goto _label)))))

(fn `PlayCutsceneSubtitle`
  (bind _csmanager (`self.CSManager`))
  (bind _subtitletextarray (`self.SubtitleTextArray`))
  (bind _subtitleindex (`self.SubtitleIndex`))
  (bind _assubtitle (cast `/Game/Bullied_VR/Blueprints/Subtitle` (`self.PSubtitleRef`)))
  (`/Engine/EditorBlueprintResources/StandardMacros.CompareInt` _subtitleindex (- (`KismetArrayLibrary.Array_Length` _subtitletextarray) 1)
    (:`>`
      (set `/Game/Bullied_VR/Blueprints/BP_MotionControllerPawnFPS.DisableMotion` false (`self.MPawnRef`))
      (`/Game/Bullied_VR/Blueprints/Subtitle.DisplaySubtitleText` _assubtitle false)
      (set `self.SubtitleIndex` 0)
      (set `self.AudioIndex` 0)
      (set `self.IsPlayingCutscene` false)
      (if (`self.StartChoiceAfter`)
        (`/Game/Bullied_VR/Blueprints/BP_Choice_Trigger_Box.StartChoiceSelection` (`/Game/Bullied_VR/Blueprints/BP_ChoiceSubtitleManager.CTB` _csmanager) (`self.ChoiceArray`) true)
        (set `self.StartChoiceAfter` false)
        (else
          (set `/Game/Bullied_VR/Blueprints/BP_ChoiceSubtitleManager.IsPlaying` false _csmanager))))
    (:`==`
      (`/Game/Bullied_VR/Blueprints/Subtitle.SetSubtitleText` _assubtitle (`|GetArrayItem` _subtitletextarray _subtitleindex) :!label _label)
      (`/Game/Bullied_VR/Blueprints/Subtitle.DisplaySubtitleText` _assubtitle true)
      (`/Engine/EditorBlueprintResources/StandardMacros.IncrementInt` _subtitleindex))
    (:`<`
      (goto _label))))

(fn `SetInteractText`
  (params (`Text Array` :type "Array of String") (`Has Audio` :type Boolean))
  (`KismetArrayLibrary.Array_Clear` (`self.InteractTextArray`))
  (`KismetArrayLibrary.Array_Clear` (`self.SubtitleTextArray`))
  (if `Has Audio`
    (set `self.SubtitleTextArray` `Text Array`)
    (else
      (set `self.InteractTextArray` `Text Array`))))

(fn `SetSubtitleText`
  (params (`String Table Name` :type Name))
  (bind _subtitletextarray (`self.SubtitleTextArray`))
  (`KismetArrayLibrary.Array_Clear` _subtitletextarray)
  (for (_ _array_index) (`KismetStringTableLibrary.GetKeysFromStringTable` `String Table Name`)
    (`KismetArrayLibrary.Array_Add` _subtitletextarray (`KismetTextLibrary.Conv_TextToString` (`KismetTextLibrary.TextFromStringTable` `String Table Name` (`KismetStringLibrary.Conv_IntToString` _array_index))))))

(fn `StartAIInteractionText`
  (params (`Text Array` :type "Array of String") (InteractingAI :type "Actor Object Reference"))
  (set `self.InteractingAI` InteractingAI)
  (`self.SetInteractText` `Text Array`)
  (bind _asbp_motion_controller_pawn_fps (cast `/Game/Bullied_VR/Blueprints/BP_MotionControllerPawnFPS` (`Controller.K2_GetPawn` (`GameplayStatics.GetPlayerController` 0))))
  (set `self.PSubtitleRef` (`/Game/Bullied_VR/Blueprints/BP_MotionControllerPawnFPS.SubtitleWidget` _asbp_motion_controller_pawn_fps))
  (set `self.MPawnRef` _asbp_motion_controller_pawn_fps)
  (set `self.IsInteracting` true))

(fn `StartInteractionText`
  (params (`Text Array` :type "Array of String") (HasAudio :type Boolean))
  (`self.SetInteractText` `Text Array` HasAudio)
  (bind _asbp_motion_controller_pawn_fps (cast `/Game/Bullied_VR/Blueprints/BP_MotionControllerPawnFPS` (`Controller.K2_GetPawn` (`GameplayStatics.GetPlayerController` 0))))
  (set `self.PSubtitleRef` (`/Game/Bullied_VR/Blueprints/BP_MotionControllerPawnFPS.SubtitleWidget` _asbp_motion_controller_pawn_fps))
  (set `self.MPawnRef` _asbp_motion_controller_pawn_fps)
  (set `self.IsInteracting` true)
  (if (not HasAudio)
    (`self.IterateText`)))

(fn `StartSubtitleSequence`
  (params (SubInfo :type "/Game/Bullied_VR/Blueprints/SubtitleInfo Structure") (`Disable Motion` :type Boolean))
  (bind (_audioarray _stringtableref) (break `/Game/Bullied_VR/Blueprints/SubtitleInfo` SubInfo))
  (bind _actorsinscene (`self.ActorsInScene`))
  (if (not (`self.IsPlayingCutscene`))
    (`self.SetSubtitleText` (`KismetTextLibrary.StringTableIdAndKeyFromText` _stringtableref))
    (bind _output_get (set `self.Audio` _audioarray))
    (`KismetArrayLibrary.Array_Clear` _actorsinscene)
    (for _array_element _output_get
      (`KismetArrayLibrary.Array_Add` _actorsinscene (`.SoundLocation_8_C278C2E049A76481885BB89AEB37B2E2` (break `/Game/Bullied_VR/Blueprints/SoundStruct` _array_element))))
    (set `self.IsPlayingCutscene` true)
    (bind _asbp_motion_controller_pawn_fps (cast `/Game/Bullied_VR/Blueprints/BP_MotionControllerPawnFPS` (`Controller.K2_GetPawn` (`GameplayStatics.GetPlayerController` 0))))
    (set `self.PSubtitleRef` (`/Game/Bullied_VR/Blueprints/BP_MotionControllerPawnFPS.SubtitleWidget` _asbp_motion_controller_pawn_fps))
    (set `self.MPawnRef` _asbp_motion_controller_pawn_fps)
    (set `/Game/Bullied_VR/Blueprints/BP_MotionControllerPawnFPS.DisableMotion` `Disable Motion` _asbp_motion_controller_pawn_fps)))

(fn `UserConstructionScript`)