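; Trigger actor for the school hallway that starts a sky light special effect when the player enters its box.
; On Tick, an overlap hides the actor, disables its collision and turns the sky light dim red.
; BeginPlay records the original color and intensity, which ResetSkyLight restores before destroying the actor; nothing here calls it.
; The color-cycling SpecialFXUpdate is disconnected, and SpecialFXEnd and BlurCamera are empty.
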(event `self.ReceiveBeginPlay`
  ;[1 1 1] Record all of the original values to revert to once SPFX is over
  (`self.Record_OriginalFX`))

(event `self.ReceiveTick`
  (params (DeltaSeconds :type "Float (single-precision)"))
  (`|ExecutionSequence`
    (:`then_0`
      ;[1 1 1] Hide this actor once collided
      (if (`PrimitiveComponent.IsOverlappingActor` (`self.BoxCollision`) (`self.PlayerMC_Ref`))
        (`self.SetActorHiddenInGame` true)
        (`self.SetActorEnableCollision` false)
        (`self.DarkenRed_FX`)))))

(fn `BlurCamera`)

(fn `DarkenRed_FX`
  (bind _lightcomponent (`SkyLight.LightComponent` (`self.SkyLightRef`)))
  (`SkyLightComponent.SetLightColor` _lightcomponent (make `LinearColor` 255.0 0.0 0.0 (`.A` (break `LinearColor` (`LightComponentBase.GetLightColor` (`SkyLight.LightComponent` (`self.SkyLightRef`)))))))
  (`SkyLightComponent.SetIntensity` _lightcomponent 0.2))

(fn `Record_OriginalFX`
  (bind _lightcomponent (`SkyLight.LightComponent` (`self.SkyLightRef`)))
  (set `self.SkyLight_OriginalColor` (`LightComponentBase.GetLightColor` _lightcomponent))
  (set `self.SkyLight_OriginalIntensity` (`LightComponentBase.Intensity` _lightcomponent)))

(fn `ResetSkyLight`
  (bind _lightcomponent (`SkyLight.LightComponent` (`self.SkyLightRef`)))
  (`SkyLightComponent.SetLightColor` _lightcomponent (`self.SkyLight_OriginalColor`))
  (`SkyLightComponent.SetIntensity` _lightcomponent (`self.SkyLight_OriginalIntensity`))
  (`self.K2_DestroyActor`))

(fn `SpecialFX_End`)

(fn `SpecialFX_Update`
  (locals (SkyLight_R :type "Float (double-precision)") (SkyLight_G :type "Float (double-precision)") (SkyLight_B :type "Float (double-precision)") (SkyLight_A :type "Float (double-precision)"))
  (bind (_r _g _b) (break `LinearColor` (`LightComponentBase.GetLightColor` (`SkyLight.LightComponent` (`self.SkyLightRef`)))))
  (bind _r_2 (break `LinearColor` (`LightComponentBase.GetLightColor` (`SkyLight.LightComponent` (`self.SkyLightRef`)))))
  (bind (_r_3 _g_2) (break `LinearColor` (`LightComponentBase.GetLightColor` (`SkyLight.LightComponent` (`self.SkyLightRef`)))))
  (bind (_r_4 _g_3 _b_2) (break `LinearColor` (`LightComponentBase.GetLightColor` (`SkyLight.LightComponent` (`self.SkyLightRef`)))))
  (bind _r_5 (break `LinearColor` (`LightComponentBase.GetLightColor` (`SkyLight.LightComponent` (`self.SkyLightRef`)))))
  (bind (_r_6 _g_4) (break `LinearColor` (`LightComponentBase.GetLightColor` (`SkyLight.LightComponent` (`self.SkyLightRef`)))))
  (`|ExecutionSequence`
    (:`then_0`
      ;[1 1 1] Check SkySphere Zenith R Increment/Decrement
      (if (>= _r_2 1.0)
        (set `self.SkyLight_R_Incre` false)
        (elif (<= _r_2 0.0)
          (set `self.SkyLight_R_Incre` true))))
    (:`then_1`
      ;[1 1 1] Check SkySphere Zenith G Increment/Decrement
      (if (>= _g_2 1.0)
        (set `self.SkyLight_G_Incre` false)
        (elif (<= _g_2 0.0)
          (set `self.SkyLight_G_Incre` true))))
    (:`then_2`
      ;[1 1 1] Check SkySphere Zenith B Increment/Decrement
      (if (>= _b_2 1.0)
        (set `self.SkyLight_B_Incre` false)
        (elif (<= _b_2 0.0)
          (set `self.SkyLight_B_Incre` true))))
    (:`then_3`
      ;[1 1 1] Set SkySphere Zenith A
      (set `local.SkyLight_A` (`.A` (break `LinearColor` (`LightComponentBase.GetLightColor` (`SkyLight.LightComponent` (`self.SkyLightRef`)))))))
    (:`then_4`
      ;[1 1 1] Set New SkySphere Zenith
      (if (`self.SkyLight_R_Incre`)
        (set `local.SkyLight_R` (+ _r_5 0.05))
        (else
          (set `local.SkyLight_R` (- _r_5 0.03)))))
    (:`then_5`
      (if (`self.SkyLight_G_Incre`)
        (set `local.SkyLight_G` (+ _g_4 0.03))
        (else
          (set `local.SkyLight_G` (- _g_4 0.01)))))
    (:`then_6`
      (if (`self.SkyLight_B_Incre`)
        (set `local.SkyLight_B` (+ _b 0.02))
        (else
          (set `local.SkyLight_B` (- _b 0.015)))))
    (:`then_7`
      ;[1 1 1] Set New SkySphere Zenith
      (`SkyLightComponent.SetLightColor` (`SkyLight.LightComponent` (`self.SkyLightRef`)) (make `LinearColor` (`local.SkyLight_R`) (`local.SkyLight_G`) (`local.SkyLight_B`) (`local.SkyLight_A`))))))

(fn `UserConstructionScript`)