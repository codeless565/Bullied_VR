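; DoorInteractible is a VR door that the player swings open and closed by pulling a trigger at a doorknob.
; When idle, Tick checks whether either motion controller from PlayerMCRef overlaps the front or back sphere with its trigger held, then toggles opening or closing.
; Tick rotates the root by a fixed, frame-rate-dependent yaw step and stops at absolute world-yaw limits, so the swing depends on placed orientation.
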(event `self.ReceiveBeginPlay`
  ;[1 1 1] Set Default Value
  (set `self.IsOpening` false)
  (set `self.IsOpened` false)
  (set `self.IsClosing` false))

(event `self.ReceiveTick`
  (params (DeltaSeconds :type "Float (single-precision)"))
  (bind _playermcref (`self.PlayerMCRef`))
  (bind _leftcontroller (`/Game/Bullied_VR/Blueprints/MotionControllerPawnFPS.LeftController` _playermcref))
  (bind _rightcontroller (`/Game/Bullied_VR/Blueprints/MotionControllerPawnFPS.RightController` _playermcref))
  ;[1 1 1] Update()
  (`|ExecutionSequence`
    (:`then_0`
      ;[1 1 1] Opening Door
      (if (`self.IsOpening`)
        (if (>= (.yaw (`SceneComponent.K2_GetComponentRotation` (`self.DefaultSceneRoot`))) 90.0)
          (set `self.IsOpened` true)
          (set `self.IsOpening` false)
          (else
            (`SceneComponent.K2_AddLocalRotation` (`self.DefaultSceneRoot`) (struct :`Yaw` 0.5) false false)))))
    (:`then_1`
      ;[1 1 1] Closing Door
      (if (`self.IsClosing`)
        (if (<= (.yaw (`SceneComponent.K2_GetComponentRotation` (`self.DefaultSceneRoot`))) 0.0)
          (set `self.IsOpened` false)
          (set `self.IsClosing` false)
          (else
            (`SceneComponent.K2_AddLocalRotation` (`self.DefaultSceneRoot`) (struct :`Yaw` -0.5) false false)))))
    (:`then_2`
      ;[1 1 1] Doorknob Interaction
      (if (not (or (`self.IsOpening`) (`self.IsClosing`)))
        (`|ExecutionSequence`
          (:`then_0`
            (if (and (or (`PrimitiveComponent.IsOverlappingActor` (`self.SphereCollision_Front`) _leftcontroller) (`PrimitiveComponent.IsOverlappingActor` (`self.SphereCollision_Back`) _leftcontroller)) (`/Game/Bullied_VR/Blueprints/MotionControllerPawnFPS.TriggerLeft_Down` _playermcref))
              (if (`self.IsOpened`) :!label _label
                (set `self.IsClosing` true)
                (else
                  (set `self.IsOpening` true)))))
          (:`then_1`
            (if (and (`/Game/Bullied_VR/Blueprints/MotionControllerPawnFPS.TriggerRight_Down` _playermcref) (or (`PrimitiveComponent.IsOverlappingActor` (`self.SphereCollision_Front`) _rightcontroller) (`PrimitiveComponent.IsOverlappingActor` (`self.SphereCollision_Back`) _rightcontroller)))
              (goto _label))))))))

(fn `UserConstructionScript`)