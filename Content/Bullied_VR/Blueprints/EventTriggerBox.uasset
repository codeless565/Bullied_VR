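; EventTriggerBox is a chained trigger volume that advances the game's checkpoint progress when the player enters it.
; On BeginPlay only the box flagged as first is enabled; others have collision, visibility and tick switched off.
; Each Tick it polls for overlap with PlayerRef, then increments CheckpointIndex in Game_Instance, enables NextEventTrigger if valid and destroys itself.
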(event `self.ReceiveBeginPlay`
  ;[1 1 1] Set enabled or not depending on previous event trigger
  (if (`self.FirstEventTrigger`)
    (`self.SetEnabled`)
    (else
      (`self.SetHidden`))))

(event `self.ReceiveTick`
  (params (DeltaSeconds :type "Float (single-precision)"))
  (bind _nexteventtrigger (`self.NextEventTrigger`))
  (bind _playerref (`self.PlayerRef`))
  ;[1 1 1] Collision with Player and spawning next event trigger
  (if (`KismetSystemLibrary.IsValid` _playerref)
    (if (`PrimitiveComponent.IsOverlappingActor` (`self.BoxCollision`) _playerref)
      (bind _asgame_instance (cast `/Game/Bullied_VR/Blueprints/Game_Instance` (`GameplayStatics.GetGameInstance`))
        (:`then`
          (bind _output_get (set `self.GameInstanceRef` _asgame_instance))
          (bind _result (`/Engine/EditorBlueprintResources/StandardMacros.IncrementInt` (`/Game/Bullied_VR/Blueprints/Game_Instance.Checkpoint_Index` _output_get))
            (:`  `
              (set `/Game/Bullied_VR/Blueprints/Game_Instance.Checkpoint_Index` _result (`self.GameInstanceRef`)))))
        (:`CastFailed`
          _))
      (if (`KismetSystemLibrary.IsValid` _nexteventtrigger)
        (`self.SetEnabled` _nexteventtrigger))
      (`self.K2_DestroyActor`))))

(fn `SetEnabled`
  (`self.SetActorEnableCollision` true)
  (`self.SetActorHiddenInGame` false)
  (`self.SetActorTickEnabled` true))

(fn `SetHidden`
  (`self.SetActorEnableCollision` false)
  (`self.SetActorHiddenInGame` true)
  (`self.SetActorTickEnabled` false))

(fn `UserConstructionScript`)