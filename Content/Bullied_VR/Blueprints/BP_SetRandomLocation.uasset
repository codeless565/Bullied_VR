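; Behavior Tree service that, on activation, writes a random reachable point near the controlled pawn to the TargetLocation blackboard key.
; A while loop tests random navigation points in a 500-unit radius for a minimum distance from the pawn.
; A passing test sets LocationNotFound to true, and nothing here clears that loop flag.
; The blackboard write makes its own random query, so the stored point is not the tested one.
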(event `self.ReceiveActivationAI`
  (params (OwnerController :type "AIController Object Reference") (ControlledPawn :type "Pawn Object Reference"))
  (bind _returnvalue (`Actor.K2_GetActorLocation` ControlledPawn))
  (bind _randomlocation (`NavigationSystem.K2_GetRandomReachablePointInRadius` _returnvalue 500.0))
  (while (`self.LocationNotFound`)
    (`/Engine/EditorBlueprintResources/StandardMacros.CompareFloat` (`KismetMathLibrary.VSize` (- _returnvalue _randomlocation)) 250.0
      (:`>`
        _)
      (:`==`
        _))
    (set `self.LocationNotFound` true))
  (`BlackboardComponent.SetValueAsVector` (`AIBlueprintHelperLibrary.GetBlackboard` OwnerController) "TargetLocation" _randomlocation))