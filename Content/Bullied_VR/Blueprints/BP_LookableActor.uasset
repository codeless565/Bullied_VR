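; BP_LookableActor is an interactable VR actor that shows interaction text when a look trigger fires.
; LookTrigger accepts only a BP_MotionControllerPawnFPS, stores it, then StartInteraction passes InteractText to TTB without audio and flags TTB as interacting.
; A HasTriggered latch blocks repeat triggers until that same pawn ends overlap with the actor.
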(event `self.ReceiveBeginPlay`)

(event `self.ReceiveActorBeginOverlap`
  (params (OtherActor :type "Actor Object Reference")))

(event `/Game/Bullied_VR/Blueprints/BP_InterfaceLookable.LookTrigger`
  (params (`Player's MCRef` :type "Actor Object Reference"))
  (if (not (`self.HasTriggered`))
    (bind _asbp_motion_controller_pawn_fps (cast `/Game/Bullied_VR/Blueprints/BP_MotionControllerPawnFPS` `Player's MCRef`))
    (set `self.PlayerMCRef` _asbp_motion_controller_pawn_fps)
    (`self.StartInteraction`)))

(event `self.ReceiveActorEndOverlap`
  (params (OtherActor :type "Actor Object Reference"))
  (if (`self.HasTriggered`)
    (if (== OtherActor (`self.PlayerMCRef`))
      (set `self.HasTriggered` false))))

(fn `StartInteraction`
  (bind _ttb (`self.TTB`))
  (`/Game/Bullied_VR/Blueprints/BP_Text_Trigger_Box.StartInteractionText` _ttb (`self.InteractText`) false)
  (set `/Game/Bullied_VR/Blueprints/BP_Text_Trigger_Box.IsInteracting` true _ttb)
  (set `self.HasTriggered` true))

(fn `UserConstructionScript`)