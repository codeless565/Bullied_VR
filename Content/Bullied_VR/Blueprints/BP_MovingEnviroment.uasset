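; Moving environment Blueprint that scrolls its parent actor in a repeating loop, presumably to simulate passing scenery.
; BeginPlay stores the parent's start location and derives an end point by scaling its world Y by -0.33, across the origin.
; Tick steps the parent 15 units toward that point without delta-time scaling, snapping it back to the start when Y reaches or passes the end.
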(event `self.ReceiveBeginPlay`
  (bind _output_get (set `self.OriginalPoint` (`self.K2_GetActorLocation` (`self.GetParentActor`))))
  (set `self.EndPoint` (* _output_get (1.0 -0.33 1.0))))

(event `self.ReceiveTick`
  (params (DeltaSeconds :type "Float (single-precision)"))
  (bind _returnvalue (`self.GetParentActor`))
  (bind _returnvalue_2 (+ (`self.K2_GetActorLocation` _returnvalue) (* (`KismetMathLibrary.Normal` (- (`self.EndPoint`) (`self.OriginalPoint`))) 15.0)))
  (`self.K2_SetActorLocation` _returnvalue _returnvalue_2 false false)
  (if (>= (.y _returnvalue_2) (.y (`self.EndPoint`)))
    (`self.K2_SetActorLocation` (`self.GetParentActor`) (`self.OriginalPoint`) false false)))

(fn `UserConstructionScript`)