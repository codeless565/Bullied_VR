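; Chainable trigger box that starts a choice or subtitle through BP_ChoiceSubtitleManager when the player overlaps it.
; Only the box flagged FirstEventTrigger starts enabled; the others start hidden, without collision or tick.
; Tick polls for overlap with PlayerRef, fires the event, enables NextEventTrigger, then destroys itself.
; Checkpoint increment logic on the game instance is present but disconnected.
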(event `self.ReceiveBeginPlay`
  ;[1 1 1] Set enabled or not depending on previous event trigger
  (if (`self.FirstEventTrigger`)
    (`self.SetEnabled`)
    (else
      (`self.SetHidden`)))
  (bind _outactors (`GameplayStatics.GetAllActorsOfClass` "/Game/Bullied_VR/Blueprints/BP_ChoiceSubtitleManager.BP_ChoiceSubtitleManager_C"))
  (for _array_element _outactors
    (set `self.CSManager` _array_element)))

(event `self.ReceiveTick`
  (params (DeltaSeconds :type "Float (single-precision)"))
  (bind _nexteventtrigger (`self.NextEventTrigger`))
  (bind _csmanager (`self.CSManager`))
  (bind _playerref (`self.PlayerRef`))
  ;[1 1 1] Collision with Player and spawning next event trigger
  (if (`KismetSystemLibrary.IsValid` _playerref)
    (if (`PrimitiveComponent.IsOverlappingActor` (`self.BoxCollision`) _playerref)
      (if (`self.IsChoice`)
        (`/Game/Bullied_VR/Blueprints/BP_ChoiceSubtitleManager.ActivateChoice` _csmanager (`self.Choice`))
        (elif (`self.IsSubtitle`)
          (`/Game/Bullied_VR/Blueprints/BP_ChoiceSubtitleManager.ActivateSubtitle` _csmanager (`self.Subtitle`) (`self.ChoiceAfterSubtitle`) (`self.Choice`))))
      (if (`KismetSystemLibrary.IsValid` _nexteventtrigger)
        (`self.SetEnabled` _nexteventtrigger))
      (`self.K2_DestroyActor`))))

(fn `SetEnabled`
  (`self.SetActorEnableCollision` true)
  (`self.SetActorHiddenInGame` false)
  (`self.SetActorTickEnabled` true))

(fn `SetHidden`
  (`self.SetActorEnableCollision` false)
  (`self.SetActorHiddenInGame` true)
  (`self.SetActorTickEnabled` false))

(fn `UserConstructionScript`)