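; AI controller for NPCs that runs the BT_NPC behavior tree and supplies it with looping patrol destinations.
; On BeginPlay it caches the controlled NPC, its waypoint count and its start location, and selects the first target.
; Each NextWaypoint call writes the next WaypointArray entry to the TargetLocation blackboard key.
; After the last waypoint it targets the start location and resets the index.
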(event `self.ReceiveBeginPlay`
  (bind _returnvalue (`self.K2_GetPawn`))
  (`self.RunBehaviorTree` "/Game/Bullied_VR/Blueprints/BT_NPC.BT_NPC")
  (bind _asnpc (cast `/Game/Bullied_VR/Blueprints/NPC` _returnvalue))
  (set `self.ControlledNPC` _asnpc)
  (set `self.WaypointLength` (`KismetArrayLibrary.Array_Length` (`/Game/Bullied_VR/Blueprints/NPC.WaypointArray` _asnpc)))
  (`self.NextWaypoint`)
  (set `self.StartLocation` (`self.K2_GetActorLocation` _returnvalue)))

(event `NextWaypoint`
  (bind _returnvalue (`AIBlueprintHelperLibrary.GetBlackboard` null))
  (bind _waypointindex (`self.WaypointIndex`))
  (`/Engine/EditorBlueprintResources/StandardMacros.CompareInt` _waypointindex (`self.WaypointLength`)
    (:`==`
      (`BlackboardComponent.SetValueAsVector` _returnvalue "TargetLocation" (`self.StartLocation`))
      (set `self.WaypointIndex` 0))
    (:`<`
      (`BlackboardComponent.SetValueAsVector` _returnvalue "TargetLocation" (`|GetArrayItem` (`/Game/Bullied_VR/Blueprints/NPC.WaypointArray` (`self.ControlledNPC`)) _waypointindex))
      (`/Engine/EditorBlueprintResources/StandardMacros.IncrementInt` _waypointindex))))

(fn `UserConstructionScript`)