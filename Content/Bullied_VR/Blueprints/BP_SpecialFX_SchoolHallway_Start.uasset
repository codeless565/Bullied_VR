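; Trigger actor for the school hallway horror effect that starts when the player overlaps its box, optionally waiting until an event trigger reference is no longer valid.
; Triggering turns the skylight dim red, hides the actor and enables the paired end trigger.
; With Distortion set, it plays a haunting sound and enables post-process blur, with Tick logic to pulse blend weight.
; FXEnd restores the recorded skylight values, zeroes the blend weight and destroys the actor.
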(event `self.ReceiveBeginPlay`
  (bind _postprocessingvolumeref (`self.PostProcessingVolumeRef`))
  ;[1 1 1] Record all of the original values to revert to once SPFX is over
  (`self.Record_OriginalFX`)
  (if (`self.Requires EventTrigger`)
    (`self.SetDisable`)
    (else
      (`self.SetEnable`)))
  (`self.SetActorHiddenInGame` false)
  (`/Engine/EditorBlueprintResources/StandardMacros.IsValid` _postprocessingvolumeref
    (:`Is Valid`
      (set `PostProcessVolume.bEnabled` false _postprocessingvolumeref))))

(event `self.ReceiveTick`
  (params (DeltaSeconds :type "Float (single-precision)"))
  (`|ExecutionSequence`
    (:`then_0`
      ;[1 1 1] Hide this actor once collided
      (if (`self.b_IsActive`)
        (if (`self.b_IsTriggered`)
          (if (`self.Distortion?`)
            (`self.FX_BlurUpdate`))
          (elif (`PrimitiveComponent.IsOverlappingActor` (`self.BoxCollision`) (`self.PlayerMC_Ref`))
            (`self.SetActorHiddenInGame` true)
            (`self.SetActorEnableCollision` false)
            (set `self.b_IsTriggered` true)
            (`self.FX_DarkenRed`)
            (`self.EnableEndTrigger`)
            (`self.SetDisable`)
            (if (`self.Distortion?`)
              (`self.FX_Blur`)
              (`GameplayStatics.PlaySound2D` "/Game/Bullied_VR/Audio/WavFile/Haunting.Haunting" 0.5))))
        (else
          (`/Engine/EditorBlueprintResources/StandardMacros.IsValid` (`self.EventTriggerRef`)
            (:`Is Not Valid`
              (`self.SetEnable`))))))))

(fn `EnableEndTrigger`
  (`/Game/Bullied_VR/Blueprints/BP_SpecialFX_SchoolHallway_End.SetEnable` (`self.SPFX_EndRef`)))

(fn `FX_Blur`
  (set `PostProcessVolume.bEnabled` true (`self.PostProcessingVolumeRef`)))

(fn `FX_BlurUpdate`
  (bind _postprocessingvolumeref (`self.PostProcessingVolumeRef`))
  (if (`self.b_BlurIncre`)
    (bind _output_get (set `PostProcessVolume.BlendWeight` (+ (`PostProcessVolume.BlendWeight` _postprocessingvolumeref) (`GameplayStatics.GetWorldDeltaSeconds`)) _postprocessingvolumeref))
    (if (>= _output_get 1.0)
      (set `self.b_BlurIncre` false))
    (else
      (bind _output_get_2 (set `PostProcessVolume.BlendWeight` (- (`PostProcessVolume.BlendWeight` _postprocessingvolumeref) (`GameplayStatics.GetWorldDeltaSeconds`)) _postprocessingvolumeref))
      (if (<= _output_get_2 0.0)
        (set `self.b_BlurIncre` true)))))

(fn `FX_DarkenRed`
  (bind _spfx_endref (`self.SPFX_EndRef`))
  (bind _lightcomponent (`SkyLight.LightComponent` (`self.SkyLightRef`)))
  (`SkyLightComponent.SetLightColor` _lightcomponent (make `LinearColor` 255.0 0.0 0.0 (`.A` (break `LinearColor` (`LightComponentBase.GetLightColor` (`SkyLight.LightComponent` (`self.SkyLightRef`)))))))
  (`SkyLightComponent.SetIntensity` _lightcomponent 0.2)
  (`/Engine/EditorBlueprintResources/StandardMacros.IsValid` _spfx_endref
    (:`Is Valid`
      (`/Game/Bullied_VR/Blueprints/BP_SpecialFX_SchoolHallway_End.SetEnable` _spfx_endref))))

(fn `FX_End`
  (bind _lightcomponent (`SkyLight.LightComponent` (`self.SkyLightRef`)))
  ;[1 1 1] Reset the lighting
  (`SkyLightComponent.SetLightColor` _lightcomponent (`self.SkyLight_OriginalColor`))
  (`SkyLightComponent.SetIntensity` _lightcomponent (`self.SkyLight_OriginalIntensity`))
  (set `PostProcessVolume.BlendWeight` 0.0 (`self.PostProcessingVolumeRef`))
  (`self.K2_DestroyActor`) ; Delete this actor once the light has been reset
)

(fn `Record_OriginalFX`
  (bind _skylightref (`self.SkyLightRef`))
  (bind _lightcomponent (`SkyLight.LightComponent` _skylightref))
  (`/Engine/EditorBlueprintResources/StandardMacros.IsValid` _skylightref
    (:`Is Valid`
      (set `self.SkyLight_OriginalColor` (`LightComponentBase.GetLightColor` _lightcomponent))
      (set `self.SkyLight_OriginalIntensity` (`LightComponentBase.Intensity` _lightcomponent)))))

(fn `SetDisable`
  (`self.SetActorEnableCollision` false)
  (set `self.b_IsActive` false))

(fn `SetEnable`
  (`self.SetActorEnableCollision` true)
  (set `self.b_IsActive` true))

(fn `UserConstructionScript`)