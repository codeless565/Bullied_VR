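; Timed event trigger that plays a voice clip and subtitle if the next event trigger stays active for longer than a set delay.
; Tick accumulates time while that trigger is visible, then plays audio at the character, sends text to the level's BP_Text_Trigger_Box and self-destructs.
; It also self-destructs if the next trigger is gone.
; Helper functions toggle visibility, collision and tick, or move the player to this actor's XY.
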(event `self.ReceiveBeginPlay`
  ;[1 1 1] Set enabled or not depending on previous event trigger
  (bind _outactors (`GameplayStatics.GetAllActorsOfClass` "/Game/Bullied_VR/Blueprints/BP_Text_Trigger_Box.BP_Text_Trigger_Box_C"))
  (for _array_element _outactors
    (set `self.TTB` _array_element)))

(event `self.ReceiveTick`
  (params (DeltaSeconds :type "Float (single-precision)"))
  (bind _nexteventtrigger (`self.NextEventTrigger`))
  ;[1 1 1] Check if Trigger is still around
  (`/Engine/EditorBlueprintResources/StandardMacros.IsValid` _nexteventtrigger
    (:`Is Valid`
      ;[1 1 1] Play Subtitle / Audio when triggered
      (if (not (`Actor.bHidden` _nexteventtrigger))
        (bind _output_get (set `self.f_elapsedTime` (+ (`self.f_elapsedTime`) (`GameplayStatics.GetWorldDeltaSeconds`))))
        (if (>= _output_get (`self.TriggerDelay`))
          (`GameplayStatics.PlaySoundAtLocation` (`self.AudioClip`) (`self.K2_GetActorLocation` (`self.Character Actor`)))
          (`/Game/Bullied_VR/Blueprints/BP_Text_Trigger_Box.StartInteractionText` (`self.TTB`) (`self.Subtitle`) false)
          (`self.K2_DestroyActor`))))
    (:`Is Not Valid`
      (`self.K2_DestroyActor`) ; If next trigger is not around, destroy self
    )))

(fn `MovePlayerToChair`
  (bind _playerref (`self.PlayerRef`))
  (`self.K2_SetActorLocation` _playerref (`KismetMathLibrary.MakeVector` (.x (`self.K2_GetActorLocation`)) (.y (`self.K2_GetActorLocation`)) (.z (`self.K2_GetActorLocation` _playerref))) false false))

(fn `SetEnabled`
  (`self.SetActorEnableCollision` true)
  (`self.SetActorHiddenInGame` false)
  (`self.SetActorTickEnabled` true))

(fn `SetHidden`
  (`self.SetActorEnableCollision` false)
  (`self.SetActorHiddenInGame` true)
  (`self.SetActorTickEnabled` false))

(fn `UserConstructionScript`)