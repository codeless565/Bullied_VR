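; Trigger volume for the VR game that ends the scene when the player enters it and moves on to the next level.
; Tick polls the box for overlap with the player reference and, on first contact, starts a held camera fade.
; A Tick-driven timer then waits for the fade time plus one second, shows the splash screen and opens the configured level, noted as the main menu.
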(event `self.ReceiveBeginPlay`
  (set `self.f_time` 0.0)
  (set `self.b_Triggered` false))

(event `self.ReceiveTick`
  (params (DeltaSeconds :type "Float (single-precision)"))
  (`|ExecutionSequence`
    (:`then_0`
      ;[1 1 1] When player collides with triggerbox, start end scene
      (if (`self.b_Triggered`)
        _
        (elif (`PrimitiveComponent.IsOverlappingActor` (`self.BoxCollision`) (`self.PlayerMC_Ref`))
          (`self.Fade Out Camera`)
          (set `self.b_Triggered` true))))
    (:`then_1`
      ;[1 1 1] Switch to Main menu after fade out
      (if (`self.b_Triggered`)
        (bind _output_get (set `self.f_time` (+ (`self.f_time`) (`GameplayStatics.GetWorldDeltaSeconds`))))
        (if (>= _output_get (+ (`self.FadeOutTime`) 1.0))
          (`StereoLayerFunctionLibrary.ShowSplashScreen`)
          (`GameplayStatics.OpenLevel` (`self.NextLevelName`)))))))

(fn `Fade Out Camera`
  (`PlayerCameraManager.StartCameraFade` (`GameplayStatics.GetPlayerCameraManager` 0) 0.0 1.0 (`self.FadeOutTime`) (`self.FadedColor`) false true))

(fn `UserConstructionScript`)