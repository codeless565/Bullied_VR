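; AI controller that runs a behavior tree and supplies its blackboard with movement points and a player target.
; On BeginPlay it stores the pawn's location as StartPosition and a random reachable point nearby as EndPosition.
; Perception updates store a perceived MotionControllerPawnFPS as Player only while that key holds no valid object.
; This controller never clears Player once set.
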(event `self.ReceiveBeginPlay`
  (bind _returnvalue (`AIBlueprintHelperLibrary.GetBlackboard` null))
  (bind _returnvalue_2 (`self.K2_GetActorLocation` (`self.K2_GetPawn`)))
  (`self.RunBehaviorTree` "/Game/Bullied_VR/Blueprints/BT.BT")
  (`BlackboardComponent.SetValueAsVector` _returnvalue "StartPosition" _returnvalue_2)
  (`BlackboardComponent.SetValueAsVector` _returnvalue "EndPosition" (`NavigationSystem.K2_GetRandomReachablePointInRadius` _returnvalue_2 500.0)))

(event `self.AIPerception.OnPerceptionUpdated`
  (params (UpdatedActors :type "Array of Actor Object Reference"))
  (bind _returnvalue (`AIBlueprintHelperLibrary.GetBlackboard` null))
  (`/Engine/EditorBlueprintResources/StandardMacros.IsValid` (`BlackboardComponent.GetValueAsObject` _returnvalue "Player")
    (:`Is Not Valid`
      (for _array_element (`AIPerceptionComponent.GetPerceivedActors` (`self.AIPerception`) null)
        (bind _asmotion_controller_pawn_fps (cast `/Game/Bullied_VR/Blueprints/MotionControllerPawnFPS` _array_element))
        (`BlackboardComponent.SetValueAsObject` _returnvalue "Player" _asmotion_controller_pawn_fps)
        (break)))))

(fn `UserConstructionScript`)