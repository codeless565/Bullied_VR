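; BP_DisappearingBlock is a minigame block that cycles between visible and hidden states, optionally starting hidden.
; Tick accumulates elapsed time, and HidePlatform turns off visibility and collision for a random duration up to MaxHiddenTime.
; UnHidePlatform restores the original scale, visibility and collision for AppearTime seconds.
; During the last tenth of that time the block shrinks by a fixed factor each frame, so the shrink rate is frame-rate dependent.
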(event `self.ReceiveBeginPlay`
  (set `self.v3_OriginalScale` (`self.GetActorRelativeScale3D`))
  (bind _output_get (set `self.b_IsHidden` (`self.StartHidden?`)))
  (if _output_get
    (`self.HidePlatform`)))

(event `self.ReceiveTick`
  (params (DeltaSeconds :type "Float (single-precision)"))
  (if (`self.b_IsHidden`)
    ;[1 1 1] Update Hidden
    (bind _output_get (set `self.f_ElapseTime` (+ (`self.f_ElapseTime`) (`GameplayStatics.GetWorldDeltaSeconds`))))
    (if (>= _output_get (`self.f_HideTime`))
      (`self.UnHidePlatform`))
    (else
      ;[1 1 1] Update UnHidden
      (bind _output_get_2 (set `self.f_ElapseTime` (+ (`self.f_ElapseTime`) (`GameplayStatics.GetWorldDeltaSeconds`))))
      (if (>= _output_get_2 (* (`self.AppearTime`) 0.9))
        (`self.SetActorRelativeScale3D` (* (`self.GetActorRelativeScale3D`) 0.9))
        (if (>= (`self.f_ElapseTime`) (`self.AppearTime`))
          (`self.HidePlatform`))))))

(fn `HidePlatform`
  (set `self.f_HideTime` (`KismetMathLibrary.RandomFloatInRange` 0.0 (`self.MaxHiddenTime`)))
  (`self.SetActorHiddenInGame` true)
  (`self.SetActorEnableCollision` false)
  (set `self.b_IsHidden` true)
  (set `self.f_ElapseTime` 0.0))

(fn `UnHidePlatform`
  (`self.SetActorRelativeScale3D` (`self.v3_OriginalScale`))
  (`self.SetActorHiddenInGame` false)
  (`self.SetActorEnableCollision` true)
  (set `self.b_IsHidden` false)
  (set `self.f_ElapseTime` 0.0))

(fn `UserConstructionScript`)